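; Player component that shows the name of the object the player is looking at on the HUD.
; BeginPlay caches the owning BP_Character and its BP_PC_OpenWorld controller, while ActivateTrace toggles a looping trace timer.
; TraceEvent line-traces forward from the camera, sending the hit actor's AC_HUDHandle ObjectName to the controller's HUD text, or clearing it otherwise.
; The camera reference is fetched lazily from the character when invalid.
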(event `self.ReceiveBeginPlay`
  (`parent.ReceiveBeginPlay`)
  ;[0 0 0] Cheap way of get the controller Ref
  (bind _asbp_character (cast `/Game/Core/Player/Logic/BP_Character` (`self.GetOwner`)))
  (set `self.PlayerRef` _asbp_character)
  (bind _asbp_pc_open_world (cast `/Game/Core/Player/Logic/BP_PC_OpenWorld` (`Pawn.GetController` (`self.PlayerRef`))))
  (`self.SetController` _asbp_pc_open_world))

(event `ActivateTrace`
  (params (bShouldActivate :type Boolean))
  ;[0 0 0] Activate and deactivate player trace
  (if bShouldActivate
    (if (not (`KismetSystemLibrary.K2_IsValidTimerHandle` (`self.TraceTimer`)))
      (bind _returnvalue (`KismetSystemLibrary.K2_SetTimerDelegate` (`|CreateDelegate` :!event `TraceEvent`) 0.1 true))
      (set `self.TraceTimer` _returnvalue))
    (elif (`KismetSystemLibrary.K2_IsValidTimerHandle` (`self.TraceTimer`))
      (`KismetSystemLibrary.K2_ClearAndInvalidateTimerHandle` (`self.TraceTimer`)))))

(event `TraceEvent`
  (bind _returnvalue (`SceneComponent.K2_GetComponentLocation` (`self.PlayerCamera`)))
  ;[0 0 0] Look for the object to interact
  (`/Engine/EditorBlueprintResources/StandardMacros.IsValid` (`self.PlayerCamera`)
    (:`Is Valid`
      (bind (_outhit _returnvalue_2) (`KismetSystemLibrary.LineTraceSingle` :`Start` (+ _returnvalue (* (`SceneComponent.GetForwardVector` (`self.PlayerCamera`)) 100)) :`End` (+ _returnvalue (* (`SceneComponent.GetForwardVector` (`self.PlayerCamera`)) (`self.DistanceToInteract`))) :`TraceChannel` "TraceTypeQuery1" :`TraceColor` (struct :`R` 0.219027 :`B` 1.0 :`A` 1.0) :`TraceHitColor` (struct :`R` 1.0 :`G` 0.62428 :`A` 1.0)))
      (if _returnvalue_2
        (bind _returnvalue_3 (`Actor.GetComponentByClass` (`.HitActor` (`GameplayStatics.BreakHitResult` _outhit)) "/Game/Core/Components/AC_HUDHandle.AC_HUDHandle_C"))
        (`/Engine/EditorBlueprintResources/StandardMacros.IsValid` _returnvalue_3
          (:`Is Valid`
            (bind _playercontrollerref (`self.PlayerControllerRef`)
              (:`then`
                (`/Game/Core/Player/Logic/BP_PC_OpenWorld.SetHUDText` _playercontrollerref (`/Game/Core/Components/AC_HUDHandle.Object Name` _returnvalue_3)))
              (:`else`)))
          (:`Is Not Valid`
            (bind _playercontrollerref_2 (`self.PlayerControllerRef`)
              (:`then`
                (`/Game/Core/Player/Logic/BP_PC_OpenWorld.SetHUDText` _playercontrollerref_2 ""))
              (:`else`))))
        (else
          (bind _playercontrollerref_3 (`self.PlayerControllerRef`)
            (:`then`
              (`/Game/Core/Player/Logic/BP_PC_OpenWorld.SetHUDText` _playercontrollerref_3 ""))
            (:`else`)))))
    (:`Is Not Valid`
      (bind _playerref (`self.PlayerRef`)
        (:`then`
          (`self.SetFollowCamera` (`/Game/Core/Player/Logic/BP_Character.Camera` _playerref)))
        (:`else`)))))

(fn `SetController`
  (params (PlayerControllerRef :type "/Game/Core/Player/Logic/BP_PC_OpenWorld Object Reference"))
  (set `self.PlayerControllerRef` PlayerControllerRef))

(fn `SetFollowCamera`
  (params (PlayerCamera :type "CameraComponent Object Reference"))
  (set `self.PlayerCamera` PlayerCamera))