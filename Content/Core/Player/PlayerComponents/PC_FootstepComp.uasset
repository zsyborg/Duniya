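; Player footstep component that tunes the volume and particle scale calculated by its parent class through two overrides.
; The volume override remaps the parent's result with a clamped range, silencing quiet values and stretching the rest up to full volume.
; The particle override multiplies the parent's scale by the owning Character's clamped velocity magnitude, so effects grow from nothing at low speed to full size at high speed.
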(fn `OverwriteCalcVolume`
  (returns (ReturnValue :type "Float (single-precision)"))
  (return (`KismetMathLibrary.MapRangeClamped` (`parent.OverwriteCalcVolume`) 0.2 1.0 0.0 1.0)))

(fn `OverwriteParticleScale`
  (returns (ReturnValue :type "Vector Structure"))
  (bind _ascharacter (cast `Character` (`self.GetOwner`)))
  (return (* (`parent.OverwriteParticleScale`) (`KismetMathLibrary.MapRangeClamped` (`KismetMathLibrary.VSize` (`Actor.GetVelocity` _ascharacter)) 200.0 3000.0 0.0 1.0))))