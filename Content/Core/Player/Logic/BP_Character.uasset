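; BP_Character is the player character, handling movement, camera look and object interaction through Enhanced Input.
; Locally controlled instances add the default mapping context, retrying until the controller cast succeeds; movement follows control yaw, and look supports sensitivity and axis inversion.
; Interact line-traces from the camera for a BP_InteractionBase, checks CanInteract locally, then forwards it through S_Interact to ServerInteraction.
; It also hands its camera to the HUD handle and debug-prints footstep volume.
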(event `self.ReceiveBeginPlay`
  (`parent.ReceiveBeginPlay`)
  (`/Game/Core/Player/PlayerComponents/PC_HUDHandle.SetFollowCamera` (`self.PC_HUDHandle`) (`self.Camera`))
  (if (`self.IsLocallyControlled`)
    (bind _asplayer_controller (cast `PlayerController` (`self.GetController`) :!label _label)
      (:`then`
        (`EnhancedInputSubsystemInterface.AddMappingContext` (pcsubsystem `EnhancedInputLocalPlayerSubsystem` _asplayer_controller) "/Game/ThirdPerson/Input/IMC_Default.IMC_Default" 0 (struct)))
      (:`CastFailed`
        (`KismetSystemLibrary.PrintString` "Cast to controller failed somehow" true true (struct :`R` 1.0 :`B` 0.098258 :`A` 1.0))
        (`KismetSystemLibrary.Delay` 1.0)
        (goto _label)))))

(event `self.PC_FootstepComp.CharacterMadeFootstepSound`
  (params (HitEvent :type "HitResult Structure") (VolumeMulti :type "Float (single-precision)") (Sound :type "AudioComponent Object Reference") (Particle :type "NiagaraSystem Object Reference") (Key :type Name))
  (`KismetSystemLibrary.PrintString` (`KismetStringLibrary.Conv_DoubleToString` VolumeMulti)))

(event `EnhancedInput|/Game/ThirdPerson/Input/Actions/IA_Move`
  (params (ActionValue :type "Vector2D Structure") (ElapsedSeconds :type "Float (double-precision)") (TriggeredSeconds :type "Float (double-precision)") (InputAction :type "InputAction Object Reference" :default "/Game/ThirdPerson/Input/Actions/IA_Move.IA_Move"))
  (bind (_forward _right) (`self.GetPawnControlVectors` false false true))
  (:`Triggered`
    (set `self.MoveAxis2D` ActionValue)
    (`self.MoveCharacter` (`self.MoveAxis2D`) false _forward _right))
  (:`Completed`
    (set `self.MoveAxis2D` (0.0 0.0))))

(event `EnhancedInput|/Game/ThirdPerson/Input/Actions/IA_Look`
  (params (ActionValue :type "Vector2D Structure") (ElapsedSeconds :type "Float (double-precision)") (TriggeredSeconds :type "Float (double-precision)") (InputAction :type "InputAction Object Reference" :default "/Game/ThirdPerson/Input/Actions/IA_Look.IA_Look"))
  (:`Triggered`
    (set `self.LookAxis2D` ActionValue)
    (set `self.FinalXAxisLook ` (* (`.Y` (`KismetMathLibrary.BreakVector2D` (* (`self.LookAxis2D`) (`self.Main sensitive`)))) (`self.mouseLEFTspeed`)))
    (set `self.FinalYAxisLook` (* (`KismetMathLibrary.BreakVector2D` (* (`self.LookAxis2D`) (`self.Main sensitive`))) (`self.mouseUPspeed`)))
    (`self.CameraRotation` (`self.Invert X`) (`self.Invert Y`) (`KismetMathLibrary.MakeVector2D` (`self.FinalXAxisLook `) (`self.FinalYAxisLook`)) 1.0))
  (:`Completed`
    (set `self.LookAxis2D` (0.0 0.0))))

(event `EnhancedInput|/Game/ThirdPerson/Input/Actions/IA_Interact`
  (params (ActionValue :type Boolean) (ElapsedSeconds :type "Float (double-precision)") (TriggeredSeconds :type "Float (double-precision)") (InputAction :type "InputAction Object Reference" :default "/Game/ThirdPerson/Input/Actions/IA_Interact.IA_Interact"))
  (bind _returnvalue (`SceneComponent.K2_GetComponentLocation` (`self.Camera`)))
  (:`Started`
    (bind (_outhit _returnvalue_2) (`KismetSystemLibrary.LineTraceSingle` :`Start` (+ _returnvalue (* (`SceneComponent.GetForwardVector` (`self.Camera`)) 100)) :`End` (+ _returnvalue (* (`SceneComponent.GetForwardVector` (`self.Camera`)) (`self.DistanceToInteract`))) :`TraceChannel` "TraceTypeQuery1" :`DrawDebugType` "ForDuration" :`TraceColor` (struct :`R` 1.0 :`B` 0.092496 :`A` 1.0) :`TraceHitColor` (struct :`R` 1.0 :`G` 0.62428 :`A` 1.0)))
    (if _returnvalue_2
      (bind _asbp_interaction_base (cast `/Game/Core/Interaction/BP_InteractionBase` (`.HitActor` (`GameplayStatics.BreakHitResult` _outhit))))
      (bind _caninteract (`/Game/Core/Interaction/BP_InteractionBase.CanInteract` _asbp_interaction_base self))
      (if _caninteract
        (`self.S_Interact` _asbp_interaction_base)))))

(event `S_Interact`
  (params (InteractionObj :type "/Game/Core/Interaction/BP_InteractionBase Object Reference"))
  (`/Game/Core/Interaction/BP_InteractionBase.Server_Interaction` InteractionObj self))

(fn `UserConstructionScript`)