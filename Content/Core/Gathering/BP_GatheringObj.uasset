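; Base multiplayer gathering node, configured from DT_Gathering by tier and type, with an empty resource-reward hook for children.
; Interaction shows a countdown widget locally and marks the node in use on the server, starting a looping timer.
; The server counts down GatheringTime while clients refresh the widget.
; On completion, it "pools" the node by shifting it vertically out of sight, then restores it after RespawnTime.
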(event `self.ReceiveBeginPlay`
  ;[0 0 0] BeginPlay
  (`parent.ReceiveBeginPlay`))

(event `self.Server_Interaction`
  (params (InteractingCharacter :type "Character Object Reference"))
  ;[0 0 0] BeginPlay
  (set `self.Interacting ActorRef` InteractingCharacter)
  (`parent.Server_Interaction` InteractingCharacter))

(event `HandleGathering`
  ;[0 0 0] Start the counter
  (bind _returnvalue (`KismetSystemLibrary.K2_SetTimerDelegate` (`|CreateDelegate` :!event `MC_GatheringTime`) (`self.ReductionTime`) true))
  (set `self.GatheringTimer` _returnvalue))

(event `AddPlayerHUD`
  ;[0 0 0] Client- Handle clinet HUD part
  (bind _asplayer_controller (cast `PlayerController` (`Pawn.GetController` (`self.Interacting ActorRef`))))
  (bind _returnvalue (`|CreateWidget` "/Game/Core/Player/UI/WBP_GatheringCounter.WBP_GatheringCounter_C" _asplayer_controller))
  (set `self.WidgetPercentage` _returnvalue)
  (if (not (`Widget.IsInViewport` (`self.WidgetPercentage`)))
    (`UserWidget.AddToViewport` (`self.WidgetPercentage`) 0))
  (set `/Game/Core/Player/UI/WBP_GatheringCounter.StartTime` (`self.Gathering Time`) (`self.WidgetPercentage`))
  (`/Game/Core/Player/UI/WBP_GatheringCounter.SetPerc` (`self.WidgetPercentage`) (`self.Gathering Time`)))

(event `MC_GatheringTime`
  ;[0 0 0] MULTICAST - Update the time on client HUD and do the collection time and deal with collection time on server side
  (if (`KismetSystemLibrary.IsServer`)
    (if (> (`self.Gathering Time`) 0.0)
      (set `self.Gathering Time` (- (`self.Gathering Time`) (`self.ReductionTime`)))
      (else
        (`self.Server_GatheringCompleted`)))
    (else
      (bind _widgetpercentage (`self.WidgetPercentage`)
        (:`then`
          (`/Game/Core/Player/UI/WBP_GatheringCounter.SetPerc` _widgetpercentage (`self.Gathering Time`)))
        (:`else`)))))

(event `Server_GatheringCompleted`
  (bind _gatheringtimer (`self.GatheringTimer`))
  ;[0 0 0] Server finished time
  (`self.GiveActorTheRessources`)
  (`self.MC_SendActorToPool`)
  (if (`KismetSystemLibrary.K2_IsValidTimerHandle` _gatheringtimer)
    (`KismetSystemLibrary.K2_ClearAndInvalidateTimerHandle` _gatheringtimer)))

(event `GiveActorTheRessources`)

(event `MC_SendActorToPool`
  ;[0 0 0] Reset object
  (if (`KismetSystemLibrary.IsServer`)
    (`KismetSystemLibrary.Delay` 0.2)
    (`self.MC_MoveObjectToPool` true)
    (`self.Server_SendActorOutOfPool`)
    (else
      (bind _widgetpercentage (`self.WidgetPercentage`) ; this basically is doing "IsServer"
        (:`then`
          (`Widget.RemoveFromParent` _widgetpercentage))
        (:`else`)))))

(event `MC_MoveObjectToPool`
  (params (bToPool :type Boolean))
  (bind (_returnvalue_x _returnvalue_y _returnvalue_z) (`KismetMathLibrary.BreakVector` (`self.K2_GetActorLocation`)))
  ;[0 0 0] Move too pool for client and server.
  (`self.K2_SetActorLocation` (`KismetMathLibrary.MakeVector` _returnvalue_x _returnvalue_y (+ _returnvalue_z (`KismetMathLibrary.SelectFloat` -1000.0 1000.0 bToPool)))))

(event `ResetVariables`
  ;[0 0 0] Server - reset variable
  (set `self.Gathering Time` (`.GatheringTime_16_5F70CE324649BAD45B25149C2F87219A` (break `/Game/Core/Gathering/Logic/Data/ST_Gathering` (`self.ObjectData`))))
  (set `self.bInUse` false))

(event `Server_SendActorOutOfPool`
  ;[0 0 0] Server- Send actor back from pool
  (`KismetSystemLibrary.Delay` (`self.RespawnTime`))
  (`self.ResetVariables`)
  (`self.MC_MoveObjectToPool` false))

(fn `HandleInteractionLocal`
  (params (InteractingActor :type "Character Object Reference"))
  (`parent.HandleInteractionLocal` InteractingActor)
  (`self.AddPlayerHUD`))

(fn `HandleInteractionServer`
  (params (InteractingActor :type "Character Object Reference"))
  (`parent.HandleInteractionServer` InteractingActor)
  (if (not (`self.bInUse`))
    (set `self.bInUse` true)
    (`self.HandleGathering`)
    (else
      (`KismetSystemLibrary.PrintString` "being gathered"))))

(fn `OnRep_bInUse`
  (`self.HandleGathering`))

(fn `OnRep_GatheringType`
  (set `self.Object Gathering Type` (`self.GatheringType`)))

(fn `OnRep_Object Mesh`
  (`StaticMeshComponent.SetStaticMesh` (`self.StaticMesh`) (`self.Object Mesh`)))

(fn `OnRep_Object Skeletal Mesh`
  (locals (LocalSkeletalMesh :type "SkeletalMeshComponent Object Reference"))
  (bind _returnvalue (`AddComponent|NODE_AddSkeletalMeshComponent-1` :`bManualAttachment` true :`RelativeTransform` (`KismetMathLibrary.MakeTransform` (0.0 0.0 0.0))))
  (set `local.LocalSkeletalMesh` _returnvalue)
  (`SceneComponent.K2_AttachToComponent` (`local.LocalSkeletalMesh`) (`self.DefaultSceneRoot`) "None" "KeepRelative" "KeepRelative" "KeepRelative" true)
  (set `SkeletalMeshComponent.SkeletalMeshAsset` (`self.Object Skeletal Mesh`) (`local.LocalSkeletalMesh`))
  (`SceneComponent.K2_SetRelativeTransform` (`local.LocalSkeletalMesh`) (`self.ObjectTransform`) false false))

(fn `OnRep_ObjectName`
  (`self.SetObjectName` (`self.ObjectName`)))

(fn `OnRep_Tier`
  (set `self.Base ObjectTier` (`self.Tier`)))

(fn `SetObjectDefaults`
  (locals (LocalSkeletalMesh :type "SkeletalMeshComponent Object Reference") (LocalObjectTransform :type "Transform Structure"))
  (bind (_collectedobjname _gatheringtype _quantitymin _quantitymax _lvlrequired _gatheringtime _objectmesh _objectskeletal _objecttransform) (break `/Game/Core/Gathering/Logic/Data/ST_Gathering` (`self.ObjectData`)))
  (bind _returnvalue (`|GetDataTableRow` "/Game/Core/Gathering/Logic/Data/DT_Gathering.DT_Gathering" (`KismetStringLibrary.Conv_StringToName` (`KismetTextLibrary.Conv_TextToString` (`|FormatText` "{0}.{1}" (`self.Base ObjectTier`) (`|GetEnumeratorNameAsString` (`self.Object Gathering Type`))))))
    (:`then`
      (set `self.ObjectData` _returnvalue)
      (set `self.Collected Obj Name` _collectedobjname)
      (set `self.ObjectTransform` _objecttransform)
      (set `self.Object Gathering Type` _gatheringtype)
      (set `self.Quantity Min` _quantitymin)
      (set `self.Quantity Max` _quantitymax)
      (set `self.Lvl Required` _lvlrequired)
      (set `self.Gathering Time` _gatheringtime)
      (if (!= _objectmesh null)
        (set `self.Object Mesh` _objectmesh)
        (`SceneComponent.K2_SetRelativeTransform` (`self.StaticMesh`) (`self.ObjectTransform`) false false)
        (else
          (set `self.Object Skeletal Mesh` _objectskeletal))))))

(fn `SetObjectName`
  (params (`Object Name` :type Text))
  (set `/Game/Core/Components/AC_HUDHandle.Object Name` `Object Name` (`self.AC_HUDHandle`)))

(fn `UserConstructionScript`
  (set `self.GatheringType` (`self.Object Gathering Type`))
  (set `self.Tier` (`self.Base ObjectTier`))
  (set `self.ObjectName` (`self.Base Object Name`))
  (`self.SetObjectDefaults`))