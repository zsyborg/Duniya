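; AC_HUDHandle is an actor component that switches on a HUD-related trace on a player pawn when it comes near the owning actor.
; A looping half-second timer set on BeginPlay drives proximity polling, with PlayerChecker running a multi-sphere pawn trace around the owner's offset location.
; Hit actors with a PC_HUDHandle component get ActivateTrace enabled.
; The last such actor is cached and deactivated on an empty sweep or a hit lacking that component.
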(event `self.ReceiveBeginPlay`
  (`KismetSystemLibrary.K2_SetTimerDelegate` (`|CreateDelegate` :!event `PlayerChecker`) 0.5 true))

(event `PlayerChecker`
  (bind _returnvalue (+ (`Actor.K2_GetActorLocation` (`self.GetOwner`)) (`self.AdjustmentLocation`)))
  ;[0 0 0] MulticastCall
  ;[0 0 0] Look for a player pawn to activate the trace on him
  (bind (_outhits _returnvalue_2) (`KismetSystemLibrary.SphereTraceMultiForObjects` _returnvalue _returnvalue (`self.InteractionRadius`) (`|MakeArray` "ObjectTypeQuery3" :!type "EObjectTypeQuery Enum")))
  (if _returnvalue_2
    ;[0 0 0] Activating player trace
    (for _array_element _outhits
      (bind (_bblockinghit _binitialoverlap _time _distance _location _impactpoint _normal _impactnormal _physmat _hitactor) (`GameplayStatics.BreakHitResult` _array_element))
      (bind _returnvalue_3 (`Actor.GetComponentByClass` _hitactor "/Game/Core/Player/PlayerComponents/PC_HUDHandle.PC_HUDHandle_C"))
      (`/Engine/EditorBlueprintResources/StandardMacros.IsValid` _returnvalue_3
        (:`Is Valid`
          (set `self.Hit Actor` _hitactor)
          (`/Game/Core/Player/PlayerComponents/PC_HUDHandle.ActivateTrace` _returnvalue_3 true))
        (:`Is Not Valid`
          (bind _hit_actor (`self.Hit Actor`)
            (:`then`
              (`/Game/Core/Player/PlayerComponents/PC_HUDHandle.ActivateTrace` (`Actor.GetComponentByClass` _hit_actor "/Game/Core/Player/PlayerComponents/PC_HUDHandle.PC_HUDHandle_C") false)
              (set `self.Hit Actor` null))
            (:`else`)))))
    (else
      ;[0 0 0] deactivating player trace
      (bind _hit_actor_2 (`self.Hit Actor`)
        (:`then`
          (`/Game/Core/Player/PlayerComponents/PC_HUDHandle.ActivateTrace` (`Actor.GetComponentByClass` _hit_actor_2 "/Game/Core/Player/PlayerComponents/PC_HUDHandle.PC_HUDHandle_C") false)
          (set `self.Hit Actor` null))
        (:`else`)))))